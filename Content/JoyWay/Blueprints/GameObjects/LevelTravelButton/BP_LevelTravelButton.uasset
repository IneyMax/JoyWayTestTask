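; BP_LevelTravelButton is a labeled trigger that sends the player to another level.
; When a BP_PlayerPawn overlaps its Capsule, it opens LevelName with absolute travel and passes DestinationTag as the options string.
; The construction script copies ButtonText to the TextRenderMassege label.
; An open-by-object-reference node using Level is present but never runs.
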(event OnComponentBeginOverlap(Capsule)
  (params (OverlappedComponent :type Primitive%20Component%20Object%20Reference) (OtherActor :type Actor%20Object%20Reference) (OtherComp :type Primitive%20Component%20Object%20Reference) (OtherBodyIndex :type Integer) (bFromSweep :type Boolean) (SweepResult :type Hit%20Result%20Structure%20%28by%20ref%29))
  (Utilities|Casting|CastToBP_PlayerPawn OtherActor)
  (Game|OpenLevel(byName) (Variables|Default|GetLevel%20Name) true (Variables|Default|GetDestinationTag)))

(fn ConstructionScript
  (Rendering|Components|TextRender|SetText (Variables|Default|GetTextRenderMassege) (Variables|Default|GetButtonText)))