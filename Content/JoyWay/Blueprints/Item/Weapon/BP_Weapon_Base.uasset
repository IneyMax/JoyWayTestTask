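; Base weapon actor that fires ammo projectiles from its launch point while active, drawing ammo from an inventory component.
; Tick shoots whenever use is on, no shot-delay or reload timer runs and ammo remains, then removes one item and reloads once the clip capacity is reached.
; Each projectile gets the ammo's config with weapon damage added.
; Ammo swaps are limited to an allowed list, and the weapon is destroyed with its owner.
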(event Custom|OnOwnerDestroyed
  (params (DestroyedActor :type Actor%20Object%20Reference))
  (Actor|DestroyActor))

(event Custom|ClearReloadTimer
  (Utilities|Time|ClearandInvalidateTimerbyHandle (Variables|Default|GetReloadTimer)))

(event Custom|ClearShotDelayTimer
  (Utilities|Time|ClearandInvalidateTimerbyHandle (Variables|Default|GetShotDelayTimer)))

(event EventActivate
  (Variables|Default|SetbIsUse true))

(event EventSetInventoryRef
  (params (InventoryComponent :type BP%20Inventory%20Component%20Object%20Reference))
  (Variables|Default|SetInventory%20Component InventoryComponent))

(event EventTick
  (params (DeltaSeconds :type Float%20%28single-precision%29))
  (if (CallFunction|CheckCanShoot)
    (CallFunction|Shot)
    (Class|InventoryComponent|RemoveInventoryItem (Variables|Default|GetInventory%20Component) (Variables|Default|GetAmmoItem) 1)
    (bind _result (Math|Integer|IncrementInt (Variables|Default|GetShotCount))
      (:%20%20
        (if (>= _result (Utilities|Struct|BreakWeaponConfig (Variables|Default|GetWeaponConfig)))
          (CallFunction|Reload))))))

(event EventBeginPlay
  (Game|BindEventtoOnDestroyed (Components|GetOwner) (EventDispatchers|CreateEvent :!event Custom|OnOwnerDestroyed)))

(event EventDeactivate
  (Variables|Default|SetbIsUse false))

(fn ConstructionScript)

(fn Shot
  (bind _launchlocation (Variables|Default|GetLaunchLocation))
  (bind _ammoitem (Variables|Default|GetAmmoItem))
  (bind _ammoconfig (Variables|/Script/JoyWayTestTask.InventoryItemAmmo|GetAmmoConfig _ammoitem))
  (bind (_speed _maxflightdistance _bulletdamage) (Utilities|Struct|BreakAmmoConfig _ammoconfig))
  (if (Utilities|IsValidClass (Variables|/Script/JoyWayTestTask.InventoryItemAmmo|GetAmmoClass (Variables|Default|GetAmmoItem)))
    (bind _returnvalue (Game|SpawnActorfromClass (Variables|/Script/JoyWayTestTask.InventoryItemAmmo|GetAmmoClass (Variables|Default|GetAmmoItem)) (Math|Transform|MakeTransform (Transformation|GetWorldLocation _launchlocation) (Transformation|GetWorldRotation _launchlocation)) "AlwaysSpawn" (Components|GetOwner) 0))
    (Class|AmmoBase|Init _returnvalue (Utilities|Struct|MakeAmmoConfig _speed _maxflightdistance (+ _bulletdamage (Utilities|Struct|BreakWeaponConfig (Variables|Default|GetWeaponConfig)))))
    (bind _returnvalue_2 (Utilities|Time|SetTimerbyEvent (EventDispatchers|CreateEvent :!event Custom|ClearShotDelayTimer) (Utilities|Struct|BreakWeaponConfig (Variables|Default|GetWeaponConfig))))
    (Variables|Default|SetShotDelayTimer _returnvalue_2)
    (else
      (Development|PrintString "NotSelectedAmmo!" true true "(R=1.000000,G=0.000000,B=0.071665,A=1.000000)"))))

(fn Reload
  (Development|PrintString "Reload...")
  (Variables|Default|SetShotCount 0)
  (bind _returnvalue (Utilities|Time|SetTimerbyEvent (EventDispatchers|CreateEvent :!event Custom|ClearReloadTimer) (Utilities|Struct|BreakWeaponConfig (Variables|Default|GetWeaponConfig))))
  (Variables|Default|SetReloadTimer _returnvalue))

(fn CheckCanShoot
  (return (Math|Boolean|ANDBoolean (Variables|Default|GetbIsUse) (not (Utilities|Time|IsValidTimerHandle (Variables|Default|GetShotDelayTimer))) (not (Utilities|Time|IsValidTimerHandle (Variables|Default|GetReloadTimer))) (> (Class|InventoryComponent|GetInventoryItemCount (Variables|Default|GetInventory%20Component) (Variables|Default|GetAmmoItem)) 0))))

(fn SetNewAmmo
  (params (NewAmmo :type Inventory%20Item%20Ammo%20Object%20Reference))
  (if (Utilities|Array|ContainsItem (Variables|Default|GetPossibleAmmo) NewAmmo)
    (Variables|Default|SetAmmoItem NewAmmo)
    (return true)
    (else
      (Variables|Default|SetAmmoItem 0)
      (return false))))