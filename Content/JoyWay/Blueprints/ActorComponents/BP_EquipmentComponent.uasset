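; Actor component that manages equipment slots, spawning the active weapon actors assigned to them.
; Event manager slot selections clear the chosen slot and destroy its actor, or cancel on reselection.
; Chosen inventory weapons spawn attached to the owner with config, ammo and inventory reference, while ammo items go to the same-numbered, default-type slot's object.
; Begin and finish use calls send Activate and Deactivate interface messages to the slot's object.
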(event Custom|OnSelectEquipmentSlot_Event
  (params (Slot :type Item%20Slot%20Structure) (Item :type Inventory%20Item%20Base%20Object%20Reference))
  (bind (_slottype _slotnumber) (Utilities|Struct|BreakItemSlot Slot))
  (if (and (== _slottype (.SlotType (Utilities|Struct|BreakItemSlot (Variables|Default|GetSelectedSlot)))) (== _slotnumber (.SlotNumber (Utilities|Struct|BreakItemSlot (Variables|Default|GetSelectedSlot)))))
    (Variables|Default|SetSelectedSlot "")
    (Default|CallOnCancelSelectWeapon (CallFunction|GetEventManager) "None")
    (else
      (bind _output_get (Variables|Default|SetSelectedSlot Slot))
      (Class|EquipmentComponent|SetSlottedItem _output_get)
      (Utilities|FlowControl|Sequence
        (:then_0
          (bind _asactor (Utilities|Casting|CastToActor (.Value (Utilities|Map|Find (Variables|Default|GetObjectsToSlots) (Variables|Default|GetSelectedSlot)))))
          (Actor|DestroyActor _asactor))
        (:then_1
          (Utilities|Map|Add (Variables|Default|GetObjectsToSlots) (Variables|Default|GetSelectedSlot) 0))))))

(event Custom|OnSelectInventoryItem_Event
  (params (Item :type Inventory%20Item%20Base%20Object%20Reference))
  (Class|EquipmentComponent|SetSlottedItem (Variables|Default|GetSelectedSlot) Item)
  (Utilities|FlowControl|Sequence
    (:then_0
      (bind _activeitem (CallFunction|CreateActiveItem Item))
      (Utilities|Map|Add (Variables|Default|GetObjectsToSlots) (Variables|Default|GetSelectedSlot) _activeitem))
    (:then_1
      (CallFunction|TrytoSetNewAmmo Item))
    (:then_2
      (Variables|Default|SetSelectedSlot ""))))

(event EventBeginPlay
  (|CallParentFunction)
  (CallFunction|InitEvents)
  (Variables|Default|SetInventoryComponent (Actor|GetComponentbyClass (Components|GetOwner) "/Game/JoyWay/Blueprints/ActorComponents/BP_InventoryComponent.BP_InventoryComponent_C")))

(fn InitEvents
  (Utilities|FlowControl|Sequence
    (:then_0
      (EventDispatchers|BindEventtoOnSelectEquipmentSlot (CallFunction|GetEventManager) (EventDispatchers|CreateEvent :!event Custom|OnSelectEquipmentSlot_Event)))
    (:then_1
      (EventDispatchers|BindEventtoOnSelectInventoryItem (CallFunction|GetEventManager) (EventDispatchers|CreateEvent :!event Custom|OnSelectInventoryItem_Event)))))

(fn BeginUseItemfromSlot
  (params (SlotKey :type Item%20Slot%20Structure%20%28by%20ref%29))
  (bind _objectstoslots (Variables|Default|GetObjectsToSlots))
  (bind (_value _returnvalue) (Utilities|Map|Find _objectstoslots SlotKey))
  (if _returnvalue
    (Class|BPIItem|Activate(Message) _value)
    (else
      (Development|PrintString "Slot not found!" true true "(R=1.000000,G=0.000000,B=0.061069,A=1.000000)"))))

(fn FinishUseItemfromSlot
  (params (SlotKey :type Item%20Slot%20Structure%20%28by%20ref%29))
  (bind _objectstoslots (Variables|Default|GetObjectsToSlots))
  (bind (_value _returnvalue) (Utilities|Map|Find _objectstoslots SlotKey))
  (if _returnvalue
    (Class|BPIItem|Deactivate(Message) _value)
    (else
      (Development|PrintString "Slot not found!" true true "(R=1.000000,G=0.018600,B=0.000000,A=1.000000)"))))

(fn CreateActiveItem
  (params (Item :type Inventory%20Item%20Base%20Object%20Reference))
  (bind _asinventory_item_weapon (Utilities|Casting|CastToInventoryItemWeapon Item)
    (:then
      (bind _newweapon (CallFunction|CreateWeapontoSlot _asinventory_item_weapon))
      (return _newweapon))
    (:CastFailed
      (return 0))))

(fn CreateWeapontoSlot
  (params (WeaponItem :type Inventory%20Item%20Weapon%20Object%20Reference))
  (bind _returnvalue (Game|SpawnActorfromClass (Variables|/Script/JoyWayTestTask.InventoryItemWeapon|GetWeaponClass WeaponItem) (Math|Transform|MakeTransform (Variables|Default|GetWeaponSpawnLocation)) "AlwaysSpawn" (Components|GetOwner) 0))
  (bind _output_get (LocalVariables|SetLNewWeapon _returnvalue))
  (Class|WeaponBase|Init _output_get (Variables|/Script/JoyWayTestTask.InventoryItemWeapon|GetWeaponConfig WeaponItem) (Variables|/Script/JoyWayTestTask.InventoryItemWeapon|GetPossibleAmmo WeaponItem))
  (Utilities|FlowControl|Sequence
    (:then_0
      (Transformation|AttachActorToActor (LocalVariables|GetLNewWeapon) (Components|GetOwner) "None" "KeepRelative" "KeepRelative" "KeepRelative" true))
    (:then_1
      (Class|BPIItem|SetInventoryRef(Message) (LocalVariables|GetLNewWeapon) (Variables|Default|GetInventoryComponent)))
    (:then_2
      (return (LocalVariables|GetLNewWeapon)))))

(fn SetAmmotoWeapon)

(fn TrytoSetNewAmmo
  (params (Item :type Inventory%20Item%20Base%20Object%20Reference))
  (bind _asinventory_item_ammo (Utilities|Casting|CastToInventoryItemAmmo Item))
  (Class|BPIWeapon|SetNewAmmo(Message) (.Value (Utilities|Map|Find (Variables|Default|GetObjectsToSlots) (Utilities|Struct|MakeItemSlot "Weapon" (.SlotNumber (Utilities|Struct|BreakItemSlot (Variables|Default|GetSelectedSlot)))))) _asinventory_item_ammo))