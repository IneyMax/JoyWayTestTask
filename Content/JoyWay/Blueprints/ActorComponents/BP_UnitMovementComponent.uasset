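; Actor component that moves and turns its owning unit from four separate directional inputs (left, right, forward, backward).
; Each setter stores its vector and recomputes a normalized movement direction from their sum, snapping the owner's rotation to face it when non-zero.
; Tick offsets the owner in world space by that direction times speed and delta time, without sweep, so movement ignores collision.
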(event Custom|UpdateMovementDirection
  (bind _output_get (Variables|Default|SetMovementDirection (Math|Vector|Normalize (+ (Variables|Default|GetLeftDirection) (Variables|Default|GetRightDirection) (Variables|Default|GetForwardDirection) (Variables|Default|GetBackwardDirection)))))
  (if (not (Math|Vector|VectorIsZero _output_get))
    (CallFunction|UpdateRotation)))

(event Custom|UpdateRotation
  (bind _returnvalue (Components|GetOwner))
  (bind _returnvalue_2 (Transformation|GetActorLocation _returnvalue))
  (Transformation|SetActorRotation (Components|GetOwner) (Math|Rotator|FindLookatRotation _returnvalue_2 (+ _returnvalue_2 (Variables|Default|GetMovementDirection)))))

(event EventTick
  (params (DeltaSeconds :type Float%20%28single-precision%29))
  (Transformation|AddActorWorldOffset (Components|GetOwner) (* (Variables|Default|GetMovementDirection) (* (Variables|Default|GetMovementSpeed) (Utilities|Time|GetWorldDeltaSeconds)))))

(fn SetLeftDirection
  (params (LeftDirection :type Vector))
  (Variables|Default|SetLeftDirection LeftDirection)
  (CallFunction|UpdateMovementDirection))

(fn SetRightDirection
  (params (RightDirection :type Vector))
  (Variables|Default|SetRightDirection RightDirection)
  (CallFunction|UpdateMovementDirection))

(fn SetForwardDirection
  (params (ForwardDirection :type Vector))
  (Variables|Default|SetForwardDirection ForwardDirection)
  (CallFunction|UpdateMovementDirection))

(fn SetBackwardDirection
  (params (BackwardDirection :type Vector))
  (Variables|Default|SetBackwardDirection BackwardDirection)
  (CallFunction|UpdateMovementDirection))