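; BP_UnitPawn_Base is a unit pawn, apparently a base class, with health tracked by a combat parameters component and shown on a health bar widget.
; On BeginPlay, InitEvents binds an event to the component's health change notification and fills the bar from current and max HP.
; The health change handler in the event graph only prints a death message when health reaches zero or below.
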(event OnHealthChanged(BP_CombatParametersComponent)
  (params (CurrenHealth :type Integer) (MaxHealth :type Integer))
  (if (<= CurrenHealth 0)
    (Development|PrintString "Death")))

(event EventBeginPlay
  (CallFunction|InitEvents))

(fn ConstructionScript)

(fn InitEvents
  (bind _bp_combatparameterscomponent (Variables|Default|GetBP_CombatParametersComponent))
  (bind (_currenhp _maxhp) (Class|CombatParametersComponent|GetHealthStats _bp_combatparameterscomponent))
  (bind _aswbp_health_bar (Utilities|Casting|CastToWBP_HealthBar (UserInterface|GetWidget (Variables|Default|GetWidget))))
  (EventDispatchers|BindEventtoOnHealthChanged (Variables|Default|GetBP_CombatParametersComponent) (EventDispatchers|CreateEvent _aswbp_health_bar :!event UpdateProgressBar))
  (Default|UpdateProgressBar _aswbp_health_bar _currenhp _maxhp))