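; Player pawn that routes input and item pickups to its movement, equipment and inventory components.
; Each move action sets its own direction vector on the unit movement component when pressed and zeroes it when released.
; UseItem begins and finishes use of the item in equipment slot 0 on press and release.
; TakeItem passes an item and count to the inventory component and returns the result of adding them.
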(event Input|ActionEvents|InputActionMoveForward
  (params (Key :type Key%20Structure :default "None"))
  ;[1 1 1] Movement
  (:Pressed
    (Default|SetForwardDirection (Variables|Default|GetBP_UnitMovementComponent) (Class|KismetMathLibrary|VectorForward)))
  (:Released
    (Default|SetForwardDirection (Variables|Default|GetBP_UnitMovementComponent) (Math|Vector|VectorZero))))

(event Input|ActionEvents|InputActionMoveBack
  (params (Key :type Key%20Structure :default "None"))
  ;[1 1 1] Movement
  (:Pressed
    (Default|SetBackwardDirection (Variables|Default|GetBP_UnitMovementComponent) (Class|KismetMathLibrary|VectorBackward)))
  (:Released
    (Default|SetBackwardDirection (Variables|Default|GetBP_UnitMovementComponent) (Math|Vector|VectorZero))))

(event Input|ActionEvents|InputActionMoveLeft
  (params (Key :type Key%20Structure :default "None"))
  ;[1 1 1] Movement
  (:Pressed
    (Default|SetLeftDirection (Variables|Default|GetBP_UnitMovementComponent) (Class|KismetMathLibrary|VectorLeft)))
  (:Released
    (Default|SetLeftDirection (Variables|Default|GetBP_UnitMovementComponent) (Math|Vector|VectorZero))))

(event Input|ActionEvents|InputActionMoveRight
  (params (Key :type Key%20Structure :default "None"))
  ;[1 1 1] Movement
  (:Pressed
    (Default|SetRightDirection (Variables|Default|GetBP_UnitMovementComponent) (Class|KismetMathLibrary|VectorRight)))
  (:Released
    (Default|SetRightDirection (Variables|Default|GetBP_UnitMovementComponent) (Math|Vector|VectorZero))))

(event Input|ActionEvents|InputActionUseItem
  (params (Key :type Key%20Structure :default "None"))
  (bind _bp_equipmentcomponent (Variables|Default|GetBP_EquipmentComponent))
  (:Pressed
    (Default|BeginUseItemfromSlot _bp_equipmentcomponent))
  (:Released
    (Default|FinishUseItemfromSlot _bp_equipmentcomponent)))

(fn ConstructionScript
  (|CallParentFunction))

(fn TakeItem
  (params (Item :type Inventory%20Item%20Base%20Object%20Reference) (Count :type Integer))
  (bind _returnvalue (Class|InventoryComponent|AddInventoryItem (Variables|Default|GetBP_InventoryComponent) Item Count))
  (return _returnvalue))