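; BP_GameModeMain is a game mode that handles initial player placement and respawning.
; New players start at the PlayerStart found using the options string, minus its first character, as the incoming name.
; SetRespawnLocation stores a transform with the given location and zero rotation.
; PlayerRestart spawns the controller's default pawn class there, ignoring collisions, and possesses it.
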(event Custom|SetRespawnLocation
  (params (Location :type Vector))
  (Variables|Default|SetRespawnTransform (Math|Transform|MakeTransform Location)))

(event Custom|PlayerRestart
  (params (PlayerController :type Controller%20Object%20Reference))
  (bind _returnvalue (Class|GameModeBase|GetDefaultPawnClassforController PlayerController))
  (bind _aspawn (Utilities|Casting|CastToPawnClass _returnvalue))
  (bind _returnvalue_2 (Game|SpawnActorfromClass _aspawn (Variables|Default|GetRespawnTransform) "AlwaysSpawn" PlayerController 0))
  (Pawn|Possess PlayerController _returnvalue_2))

(event EventHandleStartingNewPlayer
  (params (NewPlayer :type Player%20Controller%20Object%20Reference))
  (Class|GameModeBase|RestartPlayeratPlayerStart NewPlayer (Class|GameModeBase|FindPlayerStart NewPlayer (Utilities|String|GetSubstring (Variables|Default|GetOptionsString) 1 (- (Utilities|String|Len (Variables|Default|GetOptionsString)) 1)))))

(fn ConstructionScript)